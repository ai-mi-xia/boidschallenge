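; BPCharacter_Fish is a fish character Blueprint with rudimentary, apparently experimental movement logic.
; Every Tick it resets its rotation to zero, nudges itself by a small random positive local offset in X and Z, then prints its velocity for debugging.
; The offset is applied per frame without delta-time scaling, and a velocity-based AddMovementInput path is left disconnected.
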(event EventTick
  (params (DeltaSeconds :type Float%20%28single-precision%29))
  (bind _returnvalue (Math|Random|RandomFloatinRange 1.0 5.0))
  ;[1 1 1] Handle movement
  (Utilities|FlowControl|Sequence
    (:then_0
      (Transformation|SetActorRotation "0, 0, 0"))
    (:then_1
      (Transformation|AddActorLocalOffset (Math|Vector|MakeVector _returnvalue 0.0 _returnvalue) false false)
      (Development|PrintString (Utilities|String|ToString(Vector) (Transformation|GetVelocity))))))

(fn ConstructionScript)