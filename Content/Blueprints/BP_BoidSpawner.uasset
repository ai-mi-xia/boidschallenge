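; Spawner actor that populates the level with a number of fish boid characters when play begins.
; BeginPlay enables player input, then loops over the spawn count, creating each fish at a random offset scaled by a radius around the spawn point.
; Only X and Z come from that offset, so the fish spawn on a vertical plane.
; A global time dilation call is present but never runs.
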(event EventBeginPlay
  (bind _returnvalue (Math|Random|RandomUnitVector))
  (bind _spawnpoint (Variables|Default|GetSpawnPoint))
  (bind _radius (Variables|Default|GetRadius))
  (bind _returnvalue_2 (Transformation|GetWorldLocation _spawnpoint))
  (bind _returnvalue_3 (* _returnvalue _radius))
  (bind _returnvalue_4 (+ _returnvalue_2 _returnvalue_3))
  (Input|EnableInput (Game|GetPlayerController 0))
  (for _index (range 0 (Math|Float|Truncate (- (Variables|Default|GetSpawnNumber) 1.0)))
    (Game|SpawnActorfromClass "/Game/Blueprints/BPCharacter_Fish.BPCharacter_Fish_C" (Math|Transform|MakeTransform (Math|Vector|MakeVector (.x _returnvalue_4) 0.0 (.z _returnvalue_4)) "0, 0, 0" "1.000000,1.000000,1.000000") "Undefined" 0 0)))

(fn ConstructionScript)